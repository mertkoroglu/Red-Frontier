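; Player character Blueprint that handles the HUD, menus and death flow for the main character.
; BeginPlay caches the player character, adds level and health widgets, and binds to the OnUpgradePending and OnDeath events.
; A pending upgrade or the PauseGame input pauses the game and shows the matching widget with cursor and UI-only input.
; Death opens the death menu level with cursor and UI-only input.
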(event Custom|New%20Upgrade
  (CallFunction|CreateUpgradeWidget))

(event Custom|Death
  (bind _returnvalue (Game|GetPlayerController 0))
  (Game|OpenLevel(byName) "DeathMenuLevel")
  (Variables|/Script/Engine.PlayerController|SetbShowMouseCursor _returnvalue true)
  (Input|SetInputModeUIOnly _returnvalue 0 "DoNotLock"))

(event EventBeginPlay
  (CallFunction|CastCharacter)
  (CallFunction|CreateLevelandHealthWidgets)
  (EventDispatchers|BindEventtoOnUpgradePending (delegate Custom|New%20Upgrade))
  (EventDispatchers|BindEventtoOnDeath (delegate Custom|Death)))

(event Collision|EventActorBeginOverlap
  (params (OtherActor :type Actor%20Object%20Reference)))

(event Input|ActionEvents|InputActionPauseGame
  (params (Key :type Key%20Structure :default "None"))
  (:Pressed
    (CallFunction|CreatePauseMenu)))

(fn ConstructionScript)

(fn CastCharacter
  (bind _asmain_character_bp (Utilities|Casting|CastToMainCharacterBP (Game|GetPlayerCharacter 0)))
  (Variables|Default|SetMainCharacter _asmain_character_bp))

(fn CreateLevelandHealthWidgets
  (bind _returnvalue (UserInterface|CreateWidget "/Game/Dynamic/Widgets/LevelWidget.LevelWidget_C"))
  (UserInterface|Viewport|AddtoViewport _returnvalue 0)
  (bind _returnvalue_2 (UserInterface|CreateWidget "/Game/Dynamic/Widgets/HealthWidget.HealthWidget_C"))
  (UserInterface|Viewport|AddtoViewport _returnvalue_2 0))

(fn CreateUpgradeWidget
  (bind _returnvalue (Game|GetPlayerController 0))
  (bind _returnvalue_2 (UserInterface|CreateWidget "/Game/Dynamic/Widgets/UpgradeWidget.UpgradeWidget_C"))
  (UserInterface|Viewport|AddtoViewport _returnvalue_2 0)
  (Variables|/Script/Engine.PlayerController|SetbShowMouseCursor _returnvalue true)
  (Input|SetInputModeUIOnly _returnvalue 0 "DoNotLock")
  (Game|SetGamePaused true))

(fn CreatePauseMenu
  (bind _returnvalue (Game|GetPlayerController 0))
  (bind _returnvalue_2 (UserInterface|CreateWidget "/Game/Dynamic/Widgets/PauseMenuWidget.PauseMenuWidget_C"))
  (UserInterface|Viewport|AddtoViewport _returnvalue_2 0)
  (Variables|/Script/Engine.PlayerController|SetbShowMouseCursor _returnvalue true)
  (Input|SetInputModeUIOnly _returnvalue 0 "DoNotLock")
  (Game|SetGamePaused true))